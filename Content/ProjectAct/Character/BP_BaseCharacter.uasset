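; BP_BaseCharacter is a base character Blueprint that handles facing rotation and jump state for animation.
; Each Tick runs AnimationControl, which eases actor yaw toward the base aim yaw while horizontal velocity is non-zero.
; The turn takes the shortest path, scales by delta time and LerpScale, and keeps pitch and roll unchanged.
; The OnJumped event sets the IsJumping flag, which this graph never clears.
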(event `self.ReceiveTick`
  (params (DeltaSeconds :type "Float (single-precision)"))
  (`self.AnimationControl` DeltaSeconds))

(event `self.OnJumped`
  ; For Animation Control
  (set `self.IsJumping` true))

(fn `AnimationControl`
  (params (Delta :type "Float (double-precision)"))
  (locals (LerpScale :type "Float (double-precision)" :default 5.0))
  (bind (_returnvalue_roll _returnvalue_pitch _returnvalue_yaw) (`KismetMathLibrary.BreakRotator` (`self.GetBaseAimRotation`)))
  (bind (_returnvalue_roll_2 _returnvalue_pitch_2) (`KismetMathLibrary.BreakRotator` (`self.K2_GetActorRotation`)))
  (bind (_returnvalue_roll_3 _returnvalue_pitch_3 _returnvalue_yaw_2) (`KismetMathLibrary.BreakRotator` (`self.K2_GetActorRotation`)))
  (bind (_returnvalue_roll_4 _returnvalue_pitch_4 _returnvalue_yaw_3) (`KismetMathLibrary.BreakRotator` (`KismetMathLibrary.RLerp` (`KismetMathLibrary.MakeRotator` 0.0 0.0 _returnvalue_yaw_2) (`KismetMathLibrary.MakeRotator` 0.0 0.0 _returnvalue_yaw) (* Delta (`local.LerpScale`)) true)))
  (if (> (`KismetMathLibrary.VSizeXY` (`MovementComponent.Velocity` (`self.CharacterMovement`))) 0.0)
    (`self.K2_SetActorRotation` (`KismetMathLibrary.MakeRotator` _returnvalue_roll_2 _returnvalue_pitch_2 _returnvalue_yaw_3))))

(fn `UserConstructionScript`)